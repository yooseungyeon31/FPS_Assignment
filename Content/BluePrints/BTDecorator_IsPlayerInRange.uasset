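; Behavior tree decorator that passes when the AI's controlled pawn is within attack range of the player.
; PerformConditionCheckAI reads the player actor from the Blackboard and compares its 3D distance to the pawn against the AttackPlayer threshold.
; The event graph holds an unused horizontal-only variant of the check that compares against AttackPlayerRange.
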(fn PerformConditionCheckAI
  (params (OwnerController :type AI%20Controller%20Object%20Reference) (ControlledPawn :type Pawn%20Object%20Reference))
  (return (<= (Math|Vector|VectorLength (- (Transformation|GetActorLocation ControlledPawn) (Transformation|GetActorLocation (AI|BehaviorTree|GetBlackboardValueasActor (Variables|Default|GetPlayer))))) (Variables|Default|GetAttackPlayer))))