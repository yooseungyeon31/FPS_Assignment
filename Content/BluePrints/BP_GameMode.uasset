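; Game mode that spawns BP_Whisper monsters and runs a timed session, noted as three minutes.
; BeginPlay spawns ten whispers with default controllers at random points around itself, raised on Z to avoid half-buried bodies.
; Tick counts PlayTime down with an on-screen debug print.
; At zero it sets IsGameover and loops over found whispers, calling DestroyActor without an explicit target and QuitGame inside the loop.
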(event EventBeginPlay
  (bind _returnvalue (Transformation|GetActorLocation))
  (bind _returnvalue_2 (Math|Random|RandomPointinBoundingBox _returnvalue "2000.000000,2000.000000,0.000000"))
  (Variables|Default|SetWhisperCount (Variables|Default|GetWhisperCount))
  (for _index (range 0 9)
    (bind _returnvalue_3 (Game|SpawnActorfromClass "/Game/BluePrints/BP_Whisper.BP_Whisper_C" (Math|Transform|MakeTransform (Math|Vector|MakeVector (.x _returnvalue_2) (.y _returnvalue_2) (+ (.z _returnvalue_2) 9e+01)) "0, 0, 0" "1.000000,1.000000,1.000000") "AlwaysSpawn" "MultiplyWithRoot" 0 0))
    (Pawn|SpawnDefaultController _returnvalue_3)))

(event EventTick
  (params (DeltaSeconds :type Float%20%28single-precision%29))
  ;[0.15 0.15 0.15 0.5] 플레이 타임 3분
  (Variables|Default|SetPlayTime (- (Variables|Default|GetPlayTime) (Utilities|Time|GetWorldDeltaSeconds)))
  (Development|PrintString (Utilities|String|Append "플레이 시간: " (Utilities|String|ToString(Float) (Variables|Default|GetPlayTime))) true true "(R=0.053964,G=0.906729,B=1.000000,A=1.000000)" 0.0)
  (if (<= (Variables|Default|GetPlayTime) 0.0)
    ;[0.15 0.15 0.15 0.5] 게임 3분 지나면 모든 클래스 엑터를 제거해버리고 게임 종료
    (Variables|Default|SetIsGameover true)
    (bind _outactors (Actor|GetAllActorsOfClass "/Game/BluePrints/BP_Whisper.BP_Whisper_C"))
    (for _array_element _outactors
      (Actor|DestroyActor)
      (Game|QuitGame (Game|GetPlayerController 0) "Quit" false))))

(fn ConstructionScript)