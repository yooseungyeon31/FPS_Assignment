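; Behavior tree service that tells an AI pawn whether the player is within detection range.
; On activation it caches the BP_Player actor, and on tick it looks the actor up again if that reference is invalid.
; With a valid reference, each tick compares pawn-to-player distance against FindPlayerRange, writing the player to the Player blackboard key when inside and clearing it otherwise.
; Detection is distance-only, with no line-of-sight check.
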(event EventReceiveTickAI
  (params (OwnerController :type AI%20Controller%20Object%20Reference) (ControlledPawn :type Pawn%20Object%20Reference) (DeltaSeconds :type Float%20%28single-precision%29))
  (Utilities|IsValid (Variables|Default|GetBP_Player)
    (:Is%20Valid
      (if (< (Math|Vector|VectorLength (- (Transformation|GetActorLocation ControlledPawn) (Transformation|GetActorLocation (Variables|Default|GetBP_Player)))) (Variables|Default|GetFindPlayerRange))
        (Class|BTFunctionLibrary|SetBlackboardValueasObject (Variables|Default|GetPlayer) (Variables|Default|GetBP_Player))
        (else
          (Class|BTFunctionLibrary|SetBlackboardValueasObject (Variables|Default|GetPlayer)))))
    (:Is%20Not%20Valid
      (bind _returnvalue (Actor|GetActorOfClass "/Game/BluePrints/BP_Player.BP_Player_C"))
      (Variables|Default|SetBP_Player _returnvalue))))

(event EventReceiveActivationAI
  (params (OwnerController :type AI%20Controller%20Object%20Reference) (ControlledPawn :type Pawn%20Object%20Reference))
  (bind _returnvalue (Actor|GetActorOfClass "/Game/BluePrints/BP_Player.BP_Player_C"))
  (Variables|Default|SetBP_Player _returnvalue))