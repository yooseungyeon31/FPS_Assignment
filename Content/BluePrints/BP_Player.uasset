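; BP_Player is the player character, with health, a hitscan attack and a slide launch.
; Fire plays a montage, traces from screen center and damages any BP_Whisper hit; a second mesh-to-hit trace goes unused.
; AnyDamage and TrapDamage both call Damage, which subtracts fixed HP and prints it; TrapDamage also sets a timed flag.
; Slide launches along world Y, while death handling and ReduceHp are empty.
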(event Custom|TrapDamage
  ;[0.15 0.15 0.15 0.5] 장애물 닿으면 플레이어 데미지 감소 노드
  (Variables|Default|SetIsTrapDamaged true)
  (CallFunction|Damage)
  (Utilities|FlowControl|Delay 3.0)
  (Variables|Default|SetIsTrapDamaged false))

(event Game|Damage|EventAnyDamage
  (params (Damage :type Float%20%28single-precision%29) (DamageType :type Damage%20Type%20Object%20Reference) (InstigatedBy :type Controller%20Object%20Reference) (DamageCauser :type Actor%20Object%20Reference))
  ;[0.15 0.15 0.15 0.5] 플레이어 데미지
  (CallFunction|Damage))

(fn ConstructionScript)

(fn Fire
  (bind _returnvalue (Viewport|GetViewportSize))
  (bind _returnvalue_2 (Game|GetPlayerController 0))
  (bind _returnvalue_3 (/ (.y _returnvalue) 2.0))
  (bind _returnvalue_4 (/ (.x _returnvalue) 2.0))
  (bind (_worldposition _worlddirection) (Class|GameplayStatics|DeprojectScreentoWorld _returnvalue_2 (Math|Vector2D|MakeVector2D _returnvalue_4 _returnvalue_3)))
  (Animation|PlayAnimMontage "/Game/Animations/AM_Fire.AM_Fire" 1.0 "Default")
  (bind _outhit (Collision|LineTraceByChannel _worldposition (+ _worldposition (* _worlddirection 1e+03)) "TraceTypeQuery1" false 0 "None" true "(R=1.000000,G=0.000000,B=0.000000,A=1.000000)" "(R=0.000000,G=1.000000,B=0.000000,A=1.000000)" 1.0))
  (Collision|LineTraceByChannel (.location (Transformation|GetSocketTransform (Variables|Character|GetMesh) "None" "RTS_World")) (.Location (Collision|BreakHitResult _outhit)) "TraceTypeQuery1" false 0 "None" true "(R=1.000000,G=0.000000,B=0.000000,A=1.000000)" "(R=0.000000,G=1.000000,B=0.000000,A=1.000000)" 1.0)
  ;[0.15 0.15 0.15 0.5] 맞은 엑터가 몬스터니?
  (bind _asbp_whisper (Utilities|Casting|CastToBP_Whisper (.HitActor (Collision|BreakHitResult _outhit))))
  (Default|Damage _asbp_whisper))

(fn Damage
  (Variables|Default|SetPlayerHP (- (Variables|Default|GetPlayerHP) 3.0))
  (Development|PrintString (Utilities|String|Append "플레이어 체력: " (Utilities|String|ToString(Float) (Variables|Default|GetPlayerHP))) true true "(R=0.082102,G=1.000000,B=0.284899,A=1.000000)" 9999.0 "WhisperHP")
  (if (<= (Variables|Default|GetPlayerHP) 0.0)
    _))

(fn Slide
  (Character|LaunchCharacter "0.000000,1000.000000,0.000000" false false))

(fn ReduceHp)