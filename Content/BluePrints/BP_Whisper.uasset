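; BP_Whisper is an AI-driven monster character that attacks, takes damage and respawns after death.
; Damage removes one HP, playing a hit montage or triggering WhisperDeath at zero.
; Death unpossesses the AI, disables capsule collision, plays the death montage, then hides the actor.
; After a random delay, the same actor reappears at a random location with reset HP and mesh collision, then repossesses or spawns a controller.
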(event Custom|WhisperDeath
  (bind _returnvalue (Math|Random|RandomPointinBoundingBox "0, 0, 0" "2000.000000,2000.000000,0.000000"))
  (bind _returnvalue_2 (AI|GetAIController 0))
  ;[0.15 0.15 0.15 0.5] ai 를 먼저 끊어주면 죽어서도 안따라옴
  (bind _asbp_whisper_aicontroller (Utilities|Casting|CastToBP_WhisperAIController (Pawn|GetController)))
  ;;[0.15 0.15 0.15 0.5] ai 끊기
  (Pawn|UnPossess _asbp_whisper_aicontroller)
  ;[0.15 0.15 0.15 0.5] 캡슐 컴포넌트 충돌 끄는 노드
  (Collision|SetCollisionEnabled (Variables|Collision|GetCapsuleComponent) "NoCollision")
  (Animation|PlayAnimMontage "/Game/Animations/AM_Dead.AM_Dead" 1.0 "None")
  (Utilities|FlowControl|Delay 2.0)
  ;[0.15 0.15 0.15 0.5] 다시 리스폰 로직
  (Rendering|SetActorHiddenInGame true)
  (Utilities|FlowControl|Delay (Math|Random|RandomFloatinRange 1.0 5.0))
  (Transformation|SetActorLocation (Math|Vector|MakeVector (.x _returnvalue) (.y _returnvalue) (+ (.z _returnvalue) 9e+01)) false false)
  (Development|PrintString "새로운 몬스터 재스폰" true true "(R=0.000000,G=0.660000,B=1.000000,A=1.000000)" 3.0)
  ;;[0.15 0.15 0.15 0.5] 다시 살리기 . .
  (Rendering|SetActorHiddenInGame false)
  ;;;[0.15 0.15 0.15 0.5] 체력 초기화
  (Variables|Default|SetHP 1e+01)
  (Collision|SetCollisionEnabled (Variables|Character|GetMesh) "QueryAndPhysics")
  (Utilities|IsValid _returnvalue_2
    (:Is%20Valid
      (Pawn|Possess _returnvalue_2 self)
      (AI|RunBehaviorTree _returnvalue_2 "/Game/BluePrints/BT_Whisper.BT_Whisper"))
    (:Is%20Not%20Valid
      (Pawn|SpawnDefaultController))))

(fn ConstructionScript)

(fn Attack
  (Animation|PlayAnimMontage "/Game/Animations/AM_Whisper.AM_Whisper" 1.0 "Attack"))

(fn Dead
  (Animation|PlayAnimMontage "/Game/Animations/AM_Dead.AM_Dead" 1.0 "None")
  (Rendering|SetActorHiddenInGame true))

(fn Damage
  (Variables|Default|SetHP (- (Variables|Default|GetHP) 1.0))
  (Development|PrintString (Utilities|String|Append "몬스터 체력: " (Utilities|String|ToString(Float) (Variables|Default|GetHP))) true true "(R=1.000000,G=0.093481,B=0.857230,A=1.000000)" 5.0 "WhisperHP")
  (if (<= (Variables|Default|GetHP) 0)
    (Variables|Default|SetIsDead true)
    (CallFunction|WhisperDeath)
    (else
      (Animation|PlayAnimMontage "/Game/Animations/AM_Whisper.AM_Whisper" 1.0 "Damaged"))))